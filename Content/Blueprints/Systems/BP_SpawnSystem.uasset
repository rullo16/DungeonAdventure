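; Wave spawner that runs combat waves from the WaveToSpawnData map, starting after an initial delay.
; Each wave increments the counter, broadcasts the update, waits, then spawns its enemies plus a heart and bow at random points inside SpawnArea at a fixed height.
; Enemies receive the spawner as owner and are tracked in ActiveEnemies; DefeatedEnemy starts the next wave when none remain, signalling when the last wave is cleared.
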(event `self.ReceiveBeginPlay`
  (`KismetSystemLibrary.Delay` (`self.GameStartDelay`))
  (`self.IncreaseWave`))

(event `IncreaseWave`
  (bind _result (`/Engine/EditorBlueprintResources/StandardMacros.IncrementInt` (`self.CurrWave`))
    (:`  `
      (if (> (`self.CurrWave`) (`BlueprintMapLibrary.Map_Length` (`self.WaveToSpawnData`)))
        (`self.ClearedLastWave`)
        (else
          (`self.UpdateWave` _result)
          (`KismetSystemLibrary.Delay` (`self.WaveDelay`))
          (`self.SpawnWave`))))))

(fn `DefeatedEnemy`
  (params (Enemy :type "/Game/Blueprints/Characters/BP_Enemy Object Reference"))
  (`KismetArrayLibrary.Array_RemoveItem` (`self.ActiveEnemies`) Enemy)
  (if (<= (`KismetArrayLibrary.Array_Length` (`self.ActiveEnemies`)) 0)
    (`self.IncreaseWave`)))

(fn `SpawnBow`
  (params (Class :type "/Game/Blueprints/Pickups/BP_PickupBow Class Reference"))
  (bind (_origin _boxextent) (`KismetSystemLibrary.GetComponentBounds` (`self.SpawnArea`)))
  (bind (_returnvalue_x _returnvalue_y) (`KismetMathLibrary.BreakVector` (`KismetMathLibrary.RandomPointInBoundingBox` _origin _boxextent)))
  (`|SpawnActorFromClass` Class (`KismetMathLibrary.MakeTransform` (`KismetMathLibrary.MakeVector` _returnvalue_x _returnvalue_y (`self.SpawnHeight`))) "AlwaysSpawn" "MultiplyWithRoot" null null))

(fn `SpawnEnemy`
  (params (Class :type "/Game/Blueprints/Characters/BP_Enemy Class Reference"))
  (bind (_origin _boxextent) (`KismetSystemLibrary.GetComponentBounds` (`self.SpawnArea`)))
  (bind (_returnvalue_x _returnvalue_y) (`KismetMathLibrary.BreakVector` (`KismetMathLibrary.RandomPointInBoundingBox` _origin _boxextent)))
  (bind _returnvalue (`|SpawnActorFromClass` Class (`KismetMathLibrary.MakeTransform` (`KismetMathLibrary.MakeVector` _returnvalue_x _returnvalue_y (`self.SpawnHeight`))) "AlwaysSpawn" "MultiplyWithRoot" null self null))
  (`KismetArrayLibrary.Array_Add` (`self.ActiveEnemies`) _returnvalue))

(fn `SpawnHeart`
  (params (Class :type "/Game/Blueprints/Pickups/BP_PickupHeart Class Reference"))
  (bind (_origin _boxextent) (`KismetSystemLibrary.GetComponentBounds` (`self.SpawnArea`)))
  (bind (_returnvalue_x _returnvalue_y) (`KismetMathLibrary.BreakVector` (`KismetMathLibrary.RandomPointInBoundingBox` _origin _boxextent)))
  (`|SpawnActorFromClass` Class (`KismetMathLibrary.MakeTransform` (`KismetMathLibrary.MakeVector` _returnvalue_x _returnvalue_y (`self.SpawnHeight`))) "AlwaysSpawn" "MultiplyWithRoot" null null))

(fn `SpawnWave`
  (bind (_value _returnvalue) (`BlueprintMapLibrary.Map_Find` (`self.WaveToSpawnData`) (`self.CurrWave`)))
  (bind (_enemies _bow _heart) (break `/Game/Structs/S_Wave` _value))
  (if _returnvalue
    (for _array_element _enemies
      (`self.SpawnEnemy` _array_element))
    (`|ExecutionSequence`
      (:`then_0`
        (`self.SpawnHeart` _heart))
      (:`then_1`
        (`self.SpawnBow` _bow)))))

(fn `UserConstructionScript`)